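; Lift actor that carries itself upward through a one-shot sequence when something overlaps its Trigger, with no filter on the overlapping actor.
; Three chained timelines animate the Door, raise the whole actor along Z from its current location, then animate the Door again on arrival.
; Door sounds play at world origin rather than at the lift, while the travel sound plays in 2D.
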(event `self.Trigger.OnComponentBeginOverlap`
  (params (OverlappedComponent :type "PrimitiveComponent Object Reference") (OtherActor :type "Actor Object Reference") (OtherComp :type "PrimitiveComponent Object Reference") (OtherBodyIndex :type Integer) (bFromSweep :type Boolean) (SweepResult :type "HitResult Structure (by ref)"))
  (`/Engine/EditorBlueprintResources/StandardMacros.DoOnce` false
    (:`Completed`
      (`GameplayStatics.PlaySoundAtLocation` "/Game/Sounds/door.door" (0.0 0.0 0.0) (struct) 1.0 1.0 0.0 null null null)
      (bind (_direction _dooranim) (`Timeline|LiftDoor_Enter`)
        (:`Update`
          (`SceneComponent.K2_SetRelativeLocation` (`self.Door`) (* _dooranim 250.0) false false))
        (:`Finished`
          (set `self.Location` (`self.K2_GetActorLocation`))
          (`GameplayStatics.PlaySound2D` "/Game/Sounds/lift.lift" 1.0 1.0 0.0 null null)
          (bind (_direction_2 _liftanim) (`Timeline|Lift`)
            (:`Update`
              (`self.K2_SetActorLocation` (+ (`self.Location`) (`KismetMathLibrary.MakeVector` 0.0 0.0 (* _liftanim 1585.0)))))
            (:`Finished`
              (`GameplayStatics.PlaySoundAtLocation` "/Game/Sounds/door.door" (0.0 0.0 0.0) (struct) 1.0 1.0 0.0 null null null)
              (bind (_direction_3 _dooranim_2) (`Timeline|LiftDoor_Exit`)
                (:`Update`
                  (`SceneComponent.K2_SetRelativeLocation` (`self.Door`) (* _dooranim_2 250.0) false false))))))))))

(fn `UserConstructionScript`)
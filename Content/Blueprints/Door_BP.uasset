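; Door Blueprint that slides open when its entry trigger is overlapped and shuts for good once its exit trigger is overlapped.
; A timeline scaled into the door's relative location plays forward to open and reverses to close, with a sound played at the world origin each time.
; The HadBeenOpen flag latches on exit, disabling both triggers' logic, and neither trigger filters the overlapping actor.
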(event `self.TriggerEnter.OnComponentBeginOverlap`
  (params (OverlappedComponent :type "PrimitiveComponent Object Reference") (OtherActor :type "Actor Object Reference") (OtherComp :type "PrimitiveComponent Object Reference") (OtherBodyIndex :type Integer) (bFromSweep :type Boolean) (SweepResult :type "HitResult Structure (by ref)"))
  (if (not (`self.hadBeenOpen`))
    (`GameplayStatics.PlaySoundAtLocation` "/Game/Sounds/door.door" (0.0 0.0 0.0) (struct) 1.0 1.0 0.0 null null null)
    (bind (_direction _opening) (`Timeline|Door Animation` :!label _label)
      (:`Update`
        (`SceneComponent.K2_SetRelativeLocation` (`self.Door`) (* _opening 250.0) false false)))))

(event `self.TriggerExit.OnComponentBeginOverlap`
  (params (OverlappedComponent :type "PrimitiveComponent Object Reference") (OtherActor :type "Actor Object Reference") (OtherComp :type "PrimitiveComponent Object Reference") (OtherBodyIndex :type Integer) (bFromSweep :type Boolean) (SweepResult :type "HitResult Structure (by ref)"))
  (if (not (`self.hadBeenOpen`))
    (set `self.hadBeenOpen` true)
    (`GameplayStatics.PlaySoundAtLocation` "/Game/Sounds/door.door" (0.0 0.0 0.0) (struct) 1.0 1.0 0.0 null null null)
    (goto _label :!via `Reverse`)))

(fn `UserConstructionScript`)